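; BP_Track is a spline track that records a reference car's speed along its length to serve as ideal speed data.
; With RecordSpeed on, a half-second looping timer maps spline distance to car speed, stopping near the spline's end.
; Distance comes from a fixed-step linear scan for the closest spline point.
; GetIdealSpeed loops over recorded distance keys to return a speed, though its inverted-looking comparison may miss the nearest key.
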(event EventBeginPlay
  (if (Variables|Default|GetRecordSpeed)
    (Utilities|Time|SetTimerbyFunctionName 0 "Record" 0.5 true)))

(event Collision|EventActorBeginOverlap
  (params (OtherActor :type Actor%20Object%20Reference)))

(event EventTick
  (params (DeltaSeconds :type Float%20%28single-precision%29)))

(fn ConstructionScript)

(fn Record
  (bind _reference_car (Variables|Default|GetReference%20Car))
  (bind _spline (Variables|Default|GetSpline))
  (bind _returnvalue (Spline|GetLocationatDistanceAlongSpline _spline 0.0 "Local"))
  (bind _closestsplinelength (CallFunction|FindClosestPointonRoad (Transformation|GetActorLocation _reference_car)))
  (Utilities|Map|Add (Variables|Default|GetSpeedAtDistance) _closestsplinelength (Math|Vector|VectorLength (Transformation|GetVelocity _reference_car)))
  (Rendering|Debug|DrawDebugLine :LineStart _returnvalue :LineEnd (+ _returnvalue "0.000000,0.000000,500.000000") :Duration 5.0)
  (if (Math|Float|NearlyEqual(Float) _closestsplinelength (Spline|GetSplineLength _spline) 5e+02)
    (Utilities|Time|ClearTimerbyFunctionName 0 "Record")))

(fn FindClosestPointonRoad
  (params (Location :type Vector))
  (bind _spline (Variables|Default|GetSpline))
  (if (< (LocalVariables|GetDistance) (Spline|GetSplineLength _spline)) :!label _label
    (if (< (Math|Vector|Distance(Vector) Location (Spline|GetLocationatDistanceAlongSpline _spline (LocalVariables|GetDistance) "World")) (LocalVariables|GetClosestDifference))
      (LocalVariables|SetClosestDistance (LocalVariables|GetDistance))
      (LocalVariables|SetClosestDifference (Math|Vector|Distance(Vector) Location (Spline|GetLocationatDistanceAlongSpline _spline (LocalVariables|GetDistance) "World"))))
    (LocalVariables|SetDistance (+ (LocalVariables|GetDistance) 2.5e+02))
    (goto _label)
    (else
      (return (LocalVariables|GetClosestDistance)))))

(fn GetIdealSpeed
  (params (Spline%20Distance :type Float%20%28double-precision%29))
  (bind _keys (Utilities|Map|Keys (Variables|Default|GetSpeedAtDistance)))
  (LocalVariables|SetMinDelta (Math|Float|Absolute(Float) (- (Utilities|Array|Get(acopy) _keys) Spline%20Distance)))
  (LocalVariables|SetClosestSplineDisatnce (Utilities|Array|Get(acopy) _keys))
  (bind _array_element (Utilities|Array|ForEachLoopwithBreak _keys :!label _label)
    (:LoopBody
      (if (< (Math|Float|Absolute(Float) (- _array_element Spline%20Distance)) (LocalVariables|GetMinDelta))
        (goto _label Break)
        (else
          (LocalVariables|SetMinDelta (Math|Float|Absolute(Float) (- _array_element Spline%20Distance)))
          (LocalVariables|SetClosestSplineDisatnce _array_element))))
    (:Completed
      (return (.Value (Utilities|Map|Find (Variables|Default|GetSpeedAtDistance) (LocalVariables|GetClosestSplineDisatnce)))))))