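; Start/finish line trigger for the racing lap system that counts laps, times them and ends the race for the player sports car.
; The first box overlap starts the race; later ones count only if the car's sector 2 and 3 flags are set.
; Each lap closes and restarts sector timing on the pawn and replays a Timeline used as the lap clock, updating the pawn's HUD, until the final crossing calls EndOfRace.
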(event OnComponentBeginOverlap(Box)
  (params (OverlappedComponent :type Primitive%20Component%20Object%20Reference) (OtherActor :type Actor%20Object%20Reference) (OtherComp :type Primitive%20Component%20Object%20Reference) (OtherBodyIndex :type Integer) (bFromSweep :type Boolean) (SweepResult :type Hit%20Result%20Structure%20%28by%20ref%29))
  (bind _numberoflaps (Variables|Default|GetNumberOfLaps))
  (bind _lapcounter (Variables|Default|GetLapCounter))
  (bind _asplayer_sports_car_pawn (Utilities|Casting|CastToPlayerSportsCarPawn OtherActor))
  ;[1 1 1] Whether Or Not Next Lap Should Start Or Not
  ;;[1 1 1] Comment
  (if (== _lapcounter 0)
    ;[1 1 1] True Condition/ Starting Lap Timer
    (Default|StartSector1Timing _asplayer_sports_car_pawn :!label _label)
    (CallFunction|StartLapTimer)
    (Math|Integer|IncrementInt (Variables|Default|GetLapCounter)
      (:%20%20
        (Rendering|Components|TextRender|SetText (Variables|/Game/LapSystem/WB_LapCounterUI.WB_LapCounterUI_C|GetLapCounterTextBlock (Variables|/Game/VehicleTemplate/Blueprints/SportsCar/PlayerSportsCarPawn.PlayerSportsCarPawn_C|GetLapCounterUI _asplayer_sports_car_pawn)) (Utilities|Text|FormatText "Lap{LapCounter}/{NumberOfTotalLaps}" (Variables|Default|GetLapCounter) (Variables|Default|GetNumberOfLaps)))))
    (elif (and (and (Variables|/Game/VehicleTemplate/Blueprints/SportsCar/PlayerSportsCarPawn.PlayerSportsCarPawn_C|GetStartedSector2 _asplayer_sports_car_pawn) (Variables|/Game/VehicleTemplate/Blueprints/SportsCar/PlayerSportsCarPawn.PlayerSportsCarPawn_C|GetStartedSector3 _asplayer_sports_car_pawn)) (< _lapcounter _numberoflaps))
      (Default|StopSector3 _asplayer_sports_car_pawn)
      (goto _label)
      (elif (and (and (Variables|/Game/VehicleTemplate/Blueprints/SportsCar/PlayerSportsCarPawn.PlayerSportsCarPawn_C|GetStartedSector2 _asplayer_sports_car_pawn) (Variables|/Game/VehicleTemplate/Blueprints/SportsCar/PlayerSportsCarPawn.PlayerSportsCarPawn_C|GetStartedSector3 _asplayer_sports_car_pawn)) (== _lapcounter _numberoflaps))
        ;[1 1 1] End Race Logic
        (CallFunction|StopLapTimer)
        (Default|StopSector3 _asplayer_sports_car_pawn)
        (Default|EndOfRace _asplayer_sports_car_pawn)))))

(event Custom|Stop%20Lap%20Timer
  ;[1 1 1] Lap Timer Function
  (bind _laptime (Timeline|LapTimer Stop)
    (:Update
      (Variables|Default|SetLapTime _laptime)
      (Rendering|Components|TextRender|SetText (Variables|/Game/LapSystem/WB_LapCounterUI.WB_LapCounterUI_C|GetLapTime (Variables|/Game/VehicleTemplate/Blueprints/SportsCar/PlayerSportsCarPawn.PlayerSportsCarPawn_C|GetLapCounterUI (stale OnComponentBeginOverlap(Box) _asplayer_sports_car_pawn))) (Utilities|Text|FormatText "{Lap Time}" (Variables|Default|GetLapTime))))))

(event Custom|Start%20Lap%20Timer
  ;[1 1 1] Lap Timer Function
  (bind _laptime (Timeline|LapTimer PlayFromStart)
    (:Update
      (Variables|Default|SetLapTime _laptime)
      (Rendering|Components|TextRender|SetText (Variables|/Game/LapSystem/WB_LapCounterUI.WB_LapCounterUI_C|GetLapTime (Variables|/Game/VehicleTemplate/Blueprints/SportsCar/PlayerSportsCarPawn.PlayerSportsCarPawn_C|GetLapCounterUI (stale OnComponentBeginOverlap(Box) _asplayer_sports_car_pawn))) (Utilities|Text|FormatText "{Lap Time}" (Variables|Default|GetLapTime))))))

(fn ConstructionScript)